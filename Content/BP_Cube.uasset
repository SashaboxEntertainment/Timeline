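; BP_Cube is an actor that runs an elapsed-time clock and prints it as minutes and seconds.
; BeginPlay starts a looping one-second timer that increments a seconds counter on each tick.
; A helper function, SecondsToTimeString, splits the count into minutes and seconds and formats the text.
; The timer clears itself once the count reaches ten minutes.
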(event Custom|ClockTimer
  (bind _result (Math|Integer|IncrementInt (Variables|Default|GetSeconds))
    (:%20%20
      (Development|PrintString (.Result (CallFunction|SecondstoTimeString _result)) true true "(R=0.000000,G=0.660000,B=1.000000,A=1.000000)" 5.0)
      (if (== (.Minutes (CallFunction|SecondstoTimeString _result)) 10)
        (Utilities|Time|ClearandInvalidateTimerbyHandle (Variables|Default|GetTimer))))))

(event EventBeginPlay
  (bind _returnvalue (Utilities|Time|SetTimerbyEvent (delegate Custom|ClockTimer) 1.0 true))
  (Variables|Default|SetTimer _returnvalue))

(fn ConstructionScript)

(fn SecondstoTimeString
  (params (TotalSeconds :type Integer))
  (bind _returnvalue (/ TotalSeconds 60))
  (bind _returnvalue_2 (Math|Integer|%(Integer) TotalSeconds 60))
  (return _returnvalue _returnvalue_2 (Utilities|String|ToString(Text) (Utilities|Text|FormatText "{mm}:{ss}" (Utilities|Text|ToText(Integer) _returnvalue) (Utilities|Text|ToText(Integer) _returnvalue_2)))))